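; BP_Item_Book is a pickup item actor that can be collected into the inventory while something overlaps its sphere.
; The TextRender starts hidden, and the sphere's begin and end overlap events toggle its visibility and the Overlapped flag, without filtering the overlapping actor.
; PickupItem checks that flag, finds BP_Inventory through GetActorOfClass, sends AddItemMessage with BP_BaseItemClass and destroys the book.
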(event OnComponentBeginOverlap(Sphere)
  (params (OverlappedComponent :type Primitive%20Component%20Object%20Reference) (OtherActor :type Actor%20Object%20Reference) (OtherComp :type Primitive%20Component%20Object%20Reference) (OtherBodyIndex :type Integer) (bFromSweep :type Boolean) (SweepResult :type Hit%20Result%20Structure%20%28by%20ref%29))
  (Development|SetHiddeninGame (Variables|Default|GetTextRender) false false)
  (Variables|Default|SetOverlapped? true))

(event OnComponentEndOverlap(Sphere)
  (params (OverlappedComponent :type Primitive%20Component%20Object%20Reference) (OtherActor :type Actor%20Object%20Reference) (OtherComp :type Primitive%20Component%20Object%20Reference) (OtherBodyIndex :type Integer))
  (Development|SetHiddeninGame (Variables|Default|GetTextRender) true false)
  (Variables|Default|SetOverlapped? false))

(event EventBeginPlay
  (|CallParentFunction)
  (Development|SetHiddeninGame (Variables|Default|GetTextRender) true false))

(event Collision|EventActorBeginOverlap
  (params (OtherActor :type Actor%20Object%20Reference))
  (|CallParentFunction OtherActor) ; This node is disabled and will not be called.\nDrag off pins to build functionality.
)

(event EventTick
  (params (DeltaSeconds :type Float%20%28single-precision%29))
  (|CallParentFunction DeltaSeconds))

(event EventPickupItem
  (if (Variables|Default|GetOverlapped?)
    (bind _returnvalue (Actor|GetActorOfClass "/Game/TEST_TASK/Inventory_System/BP_Inventory.BP_Inventory_C"))
    (Class|BPAddItemtoInventoryInterface|AddItem(Message) _returnvalue "/Game/TEST_TASK/Items/BP_BaseItemClass.BP_BaseItemClass_C")
    (Actor|DestroyActor)))

(fn ConstructionScript
  (|CallParentFunction))